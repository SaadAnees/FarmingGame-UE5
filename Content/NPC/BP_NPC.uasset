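; NPC Blueprint with unfinished spline-movement logic, which does not move the NPC itself as wired.
; On BeginPlay it sets the first player controller's root component, not a pawn, to the Spline's location and rotation.
; The sample distance always resolves to the spline's end, since both Lerp inputs are its length.
; Tick is empty, and disconnected nodes hold unused attempts to move the actor along the spline.
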(event `self.ReceiveBeginPlay`
  (bind _returnvalue (`SplineComponent.GetSplineLength` (`self.Spline`)))
  (bind _returnvalue_2 (`KismetMathLibrary.Lerp` _returnvalue _returnvalue))
  (`SceneComponent.K2_SetRelativeLocationAndRotation` (`Actor.RootComponent` (`GameplayStatics.GetPlayerController` 0)) (`SplineComponent.GetLocationAtDistanceAlongSpline` (`self.Spline`) _returnvalue_2 "World") (`SplineComponent.GetRotationAtDistanceAlongSpline` (`self.Spline`) _returnvalue_2 "World") false false))

(event `self.ReceiveTick`
  (params (DeltaSeconds :type "Float (single-precision)")))

(fn `UserConstructionScript`)